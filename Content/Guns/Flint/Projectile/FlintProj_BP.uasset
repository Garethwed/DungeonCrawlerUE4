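; Projectile fired by the Flint gun that flies from the player's muzzle and expires after a second.
; On BeginPlay it gives its Sphere a velocity-change impulse along the player character's Muzzle forward vector, scaled by ShotStrength.
; A fast looping timer runs FlintProj, which rotates the Sphere to face the player camera with a pitch offset, billboard-style, until the projectile is destroyed.
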(event `self.ReceiveBeginPlay`
  (`KismetSystemLibrary.K2_SetTimer` null "FlintProj" 0.01 true)
  (`PrimitiveComponent.AddImpulse` (`self.Sphere`) (* (`SceneComponent.GetForwardVector` (`/Game/ThirdPersonBP/Blueprints/ThirdPersonCharacter.Muzzle` (cast `/Game/ThirdPersonBP/Blueprints/ThirdPersonCharacter` (`GameplayStatics.GetPlayerPawn` 0) :!pure true))) (`self.ShotStrength`)) "None" true)
  (`KismetSystemLibrary.Delay` 1.0)
  (`KismetSystemLibrary.K2_ClearTimer` null "FlintProj")
  (`self.K2_DestroyActor`))

(fn `FlintProj`
  (bind (_returnvalue_roll _returnvalue_pitch _returnvalue_yaw) (`KismetMathLibrary.BreakRotator` (`KismetMathLibrary.Conv_VectorToRotator` (`KismetMathLibrary.Normal` (- (`PlayerCameraManager.GetCameraLocation` (`GameplayStatics.GetPlayerCameraManager` 0)) (`self.K2_GetActorLocation`))))))
  (`SceneComponent.K2_SetWorldRotation` (`self.Sphere`) (`KismetMathLibrary.MakeRotator` _returnvalue_roll (+ _returnvalue_pitch 90.0) _returnvalue_yaw) false false))

(fn `UserConstructionScript`)