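; Bouncing fireball projectile that launches along the player character's Muzzle forward vector via a velocity-change impulse on its physics Sphere.
; Sphere hits increment a bounce counter; the third spawns an explosion and destroys the actor, which otherwise expires after a short delay.
; A fast looping timer rotates Plane and Sphere billboard-style, using camera location minus camera manager actor location rather than the fireball's position.
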(event `self.ReceiveBeginPlay`
  (`KismetSystemLibrary.K2_SetTimer` null "FaceFireball" 0.01 true)
  (`PrimitiveComponent.AddImpulse` (`self.Sphere`) (* (`SceneComponent.GetForwardVector` (`/Game/ThirdPersonBP/Blueprints/ThirdPersonCharacter.Muzzle` (cast `/Game/ThirdPersonBP/Blueprints/ThirdPersonCharacter` (`GameplayStatics.GetPlayerPawn` 0) :!pure true))) (`self.Shot Strength`)) "None" true)
  (`KismetSystemLibrary.Delay` 5.0)
  (`KismetSystemLibrary.K2_ClearTimer` null "FaceFireball")
  (`self.K2_DestroyActor`))

(event `self.Sphere.OnComponentHit`
  (params (HitComponent :type "PrimitiveComponent Object Reference") (OtherActor :type "Actor Object Reference") (OtherComp :type "PrimitiveComponent Object Reference") (NormalImpulse :type "Vector Structure") (Hit :type "HitResult Structure (by ref)"))
  (switch `int` (`self.Bounces`)
    (:`0`
      (`/Engine/EditorBlueprintResources/StandardMacros.IncrementInt` (`self.Bounces`) :!label _label))
    (:`1`
      (goto _label))
    (:`2`
      (set `self.Bounces` 0)
      (`GameplayStatics.SpawnEmitterAtLocation` "/Game/StarterContent/Particles/P_Explosion.P_Explosion" (`.Location` (`GameplayStatics.BreakHitResult` Hit)))
      (`KismetSystemLibrary.K2_ClearTimer` null "FaceFireBall")
      (`self.K2_DestroyActor`))))

(fn `FaceFireball`
  (bind _returnvalue (`GameplayStatics.GetPlayerCameraManager` 0))
  (bind (_returnvalue_roll _returnvalue_pitch _returnvalue_yaw) (`KismetMathLibrary.BreakRotator` (`KismetMathLibrary.Conv_VectorToRotator` (`KismetMathLibrary.Normal` (- (`PlayerCameraManager.GetCameraLocation` _returnvalue) (`self.K2_GetActorLocation` _returnvalue))))))
  (`SceneComponent.K2_SetWorldRotation` (`self.Plane`) (`KismetMathLibrary.MakeRotator` _returnvalue_roll (+ _returnvalue_pitch 90.0) _returnvalue_yaw) false false)
  (`SceneComponent.K2_SetWorldRotation` (`self.Sphere`) (`KismetMathLibrary.MakeRotator` _returnvalue_roll (+ _returnvalue_pitch 90.0) _returnvalue_yaw) false false))

(fn `UserConstructionScript`)