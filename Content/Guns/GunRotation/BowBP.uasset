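; BowBP is a bow pickup Actor that rotates in the level.
; Tick adds yaw to BowCollision each frame, scaled by delta time and Yawpersecond.
; Any actor overlap casts player 0's character to ThirdPersonCharacter, sets its bow and weapon picked-up flags, and assigns BowBP to its BowOnFloor variable.
; The overlap does not check which actor entered, and the pickup does not hide or destroy itself.
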(event `self.ReceiveTick`
  (params (DeltaSeconds :type "Float (single-precision)"))
  (`SceneComponent.K2_AddRelativeRotation` (`self.BowCollision`) (`KismetMathLibrary.MakeRotator` 0.0 0.0 (* DeltaSeconds (`self.yawpersecond`))) false false))

(event `self.ReceiveActorBeginOverlap`
  (params (OtherActor :type "Actor Object Reference"))
  (bind _asthird_person_character (cast `/Game/ThirdPersonBP/Blueprints/ThirdPersonCharacter` (`GameplayStatics.GetPlayerCharacter` 0)))
  (set `/Game/ThirdPersonBP/Blueprints/ThirdPersonCharacter.BowPickedUp` true _asthird_person_character)
  (set `/Game/ThirdPersonBP/Blueprints/ThirdPersonCharacter.WeaponPickedUp` true _asthird_person_character)
  (set `/Game/ThirdPersonBP/Blueprints/ThirdPersonCharacter.BowOnFloor` "BowBP_C" _asthird_person_character))

(fn `UserConstructionScript`)