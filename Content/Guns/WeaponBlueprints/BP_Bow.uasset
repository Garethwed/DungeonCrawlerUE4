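; BP_Bow is a bow weapon Blueprint that fires arrows.
; Pressing the WeaponShoot input action spawns an Arrow_BP at the MuzzleArrow component's world transform, with no cooldown, ammo or equip check in this graph.
; Tick is empty, and a leftover node that would yaw-spin the skeletal mesh is disconnected and never runs.
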(event `self.ReceiveTick`
  (params (DeltaSeconds :type "Float (single-precision)")))

(event `InputAction|WeaponShoot`
  (params (Key :type "Key Structure"))
  (:`Pressed`
    (`|SpawnActorFromClass` "/Game/Guns/Bow/Arrow/Arrow_BP.Arrow_BP_C" (`SceneComponent.K2_GetComponentToWorld` (`self.Muzzle Arrow`)) "Undefined" "OverrideRootScale" null null)))

(fn `UserConstructionScript`
  (`parent.UserConstructionScript`))