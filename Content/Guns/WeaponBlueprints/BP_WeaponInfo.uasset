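; BP_WeaponInfo is a world weapon Blueprint that the ThirdPersonCharacter can pick up and drop.
; Sphere overlap stores the character and toggles pickup eligibility; entering also enables input, while both entering and leaving set the widget visible.
; Pickup input passes the weapon to the character only when eligible, whereas drop input calls the character without that check.
; The construction script rebuilds the WeaponInfo struct, inserting the actor's own class.
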(event `self.Sphere Collision.OnComponentBeginOverlap`
  (params (OverlappedComponent :type "PrimitiveComponent Object Reference") (OtherActor :type "Actor Object Reference") (OtherComp :type "PrimitiveComponent Object Reference") (OtherBodyIndex :type Integer) (bFromSweep :type Boolean) (SweepResult :type "HitResult Structure (by ref)"))
  (bind _asthird_person_character (cast `/Game/ThirdPersonBP/Blueprints/ThirdPersonCharacter` OtherActor))
  (set `self.Char_ref` _asthird_person_character)
  (`SceneComponent.SetVisibility` (`self.Widget`) true false)
  (set `self.CanPickWeapon?` true)
  (`self.EnableInput` (`GameplayStatics.GetPlayerController` 0)))

(event `self.Sphere Collision.OnComponentEndOverlap`
  (params (OverlappedComponent :type "PrimitiveComponent Object Reference") (OtherActor :type "Actor Object Reference") (OtherComp :type "PrimitiveComponent Object Reference") (OtherBodyIndex :type Integer))
  (bind _asthird_person_character (cast `/Game/ThirdPersonBP/Blueprints/ThirdPersonCharacter` OtherActor))
  (set `self.Char_ref` _asthird_person_character)
  (`SceneComponent.SetVisibility` (`self.Widget`) true false)
  (set `self.CanPickWeapon?` false))

(event `InputAction|WeaponPickup`
  (params (Key :type "Key Structure"))
  (:`Pressed`
    (if (`self.CanPickWeapon?`)
      (`/Game/ThirdPersonBP/Blueprints/ThirdPersonCharacter.Weaponpickup` (`self.Char_ref`) self))))

(event `InputAction|WeaponDrop`
  (params (Key :type "Key Structure"))
  (:`Pressed`
    (`/Game/ThirdPersonBP/Blueprints/ThirdPersonCharacter.Weapondrop` (`self.Char_ref`) self)))

(fn `UserConstructionScript`
  (bind (_weaponinfo_weapontype _weaponinfo_weaponclass _weaponinfo_image _weaponinfo_name _weaponinfo_equipsocket _weaponinfo_unequipsocket _weaponinfo_firerate _weaponinfo_damage _weaponinfo_range) (break `/Game/Guns/WeaponBlueprints/WeaponInfo` (`self.WeaponInfo`)))
  (set `self.WeaponInfo` (make `/Game/Guns/WeaponBlueprints/WeaponInfo` _weaponinfo_weapontype (`GameplayStatics.GetObjectClass` self) _weaponinfo_image _weaponinfo_name _weaponinfo_equipsocket _weaponinfo_unequipsocket _weaponinfo_firerate _weaponinfo_damage _weaponinfo_range)))