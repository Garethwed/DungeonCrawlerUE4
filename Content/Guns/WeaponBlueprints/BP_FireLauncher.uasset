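; BP_FireLauncher is a fire launcher weapon that spins its mesh and shoots fireballs.
; Tick yaws the skeletal mesh at a set rate until StopRotation is true, provided the player is a ThirdPersonCharacter.
; WeaponShoot spawns FireBall_BP at the MuzzleFB transform, then draws a debug camera trace whose result does not steer the projectile.
; An alternative spawn aimed at a trace hit from the launcher socket is left unconnected.
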(event `self.ReceiveTick`
  (params (DeltaSeconds :type "Float (single-precision)"))
  (cast `/Game/ThirdPersonBP/Blueprints/ThirdPersonCharacter` (`GameplayStatics.GetPlayerCharacter` 0))
  (if (not (`self.StopRotation`))
    (`SceneComponent.K2_AddRelativeRotation` (`self.SkeletalMesh`) (`KismetMathLibrary.MakeRotator` 0.0 0.0 (* DeltaSeconds (`self.yawpersecond_0`))) false false)))

(event `InputAction|WeaponShoot`
  (params (Key :type "Key Structure"))
  (bind _returnvalue (`GameplayStatics.GetPlayerCameraManager` 0))
  (bind _returnvalue_2 (`self.K2_GetActorLocation` _returnvalue))
  (:`Pressed`
    (`|SpawnActorFromClass` "/Game/Guns/Fireball_Launcher/NewFolder/FireBall_BP.FireBall_BP_C" (`SceneComponent.GetSocketTransform` (`self.MuzzleFB`) "None" "RTS_World") "Undefined" "OverrideRootScale" null null)
    (bind _outhit (`KismetSystemLibrary.LineTraceSingle` :`Start` _returnvalue_2 :`End` (+ (* (`self.GetActorForwardVector` _returnvalue) 3000.0) _returnvalue_2) :`TraceChannel` "TraceTypeQuery1" :`DrawDebugType` "ForDuration"))))

(fn `UserConstructionScript`
  (`parent.UserConstructionScript`))