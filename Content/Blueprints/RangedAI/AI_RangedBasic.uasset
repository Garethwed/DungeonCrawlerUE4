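; Basic ranged enemy AI that stops and plays a throw montage when the player character enters its trigger box.
; Shoot, which has no caller here, traces from the Hips socket toward the player's mesh and spawns BP_RangedAIProj aimed at the result.
; Leaving the box triggers a delayed Reset that restores walking, re-arms the DoOnce and replays the montage if the player is back inside.
; DamagePlayer is an empty stub.
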(event `Shoot`
  (bind _returnvalue (`SceneComponent.GetSocketLocation` (`self.Mesh`) "Hips"))
  (bind (_outhit _returnvalue_2) (`KismetSystemLibrary.LineTraceSingle` :`Start` (`SceneComponent.GetSocketLocation` (`self.Mesh`) "Hips") :`End` (`SceneComponent.K2_GetComponentLocation` (`Character.Mesh` (`self.Player`))) :`TraceChannel` "TraceTypeQuery1" :`bTraceComplex` true :`DrawDebugType` "ForDuration"))
  (bind (_bblockinghit _binitialoverlap _time _distance _location _impactpoint _normal _impactnormal _physmat _hitactor _hitcomponent _hitbonename _hititem _faceindex _tracestart _traceend) (`GameplayStatics.BreakHitResult` _outhit))
  (`|SpawnActorFromClass` "/Game/Blueprints/RangedAI/BP_RangedAIProj.BP_RangedAIProj_C" (`KismetMathLibrary.MakeTransform` _returnvalue (`KismetMathLibrary.FindLookAtRotation` _returnvalue (`KismetMathLibrary.SelectVector` _impactpoint _traceend _returnvalue_2))) "Undefined" "OverrideRootScale" null null)
  (`KismetSystemLibrary.PrintString` "Hello"))

(event `self.Box.OnComponentBeginOverlap`
  (params (OverlappedComponent :type "PrimitiveComponent Object Reference") (OtherActor :type "Actor Object Reference") (OtherComp :type "PrimitiveComponent Object Reference") (OtherBodyIndex :type Integer) (bFromSweep :type Boolean) (SweepResult :type "HitResult Structure (by ref)"))
  (bind _asthird_person_character (cast `/Game/ThirdPersonBP/Blueprints/ThirdPersonCharacter` OtherActor))
  (set `self.Player` _asthird_person_character)
  (`/Engine/EditorBlueprintResources/StandardMacros.DoOnce` false :!label _label
    (:`Completed`
      (`AnimInstance.Montage_Play` (`SkeletalMeshComponent.GetAnimInstance` (`self.Mesh`)) "/Game/Blueprints/MeleeAttackAI/Anims/ThrowRangedMontage.ThrowRangedMontage" 1.0 "MontageLength" 0.0 true)
      (`CharacterMovementComponent.DisableMovement` (`self.CharacterMovement`))
      (`KismetSystemLibrary.PrintString` "playing montage"))))

(event `DamagePlayer`
  ;[1 1 1] Do damage to player here
)

(event `Reset`
  (`CharacterMovementComponent.SetMovementMode` (`self.CharacterMovement`) "MOVE_Walking" 0)
  (if (`PrimitiveComponent.IsOverlappingActor` (`self.Box`) (`self.Player`))
    (`AnimInstance.Montage_Play` (`SkeletalMeshComponent.GetAnimInstance` (`self.Mesh`)) "/Game/Blueprints/MeleeAttackAI/Anims/ThrowRangedMontage.ThrowRangedMontage" 1.0 "MontageLength" 0.0 true)
    (goto _label :!via `Reset`)
    (else
      (goto _label :!via `Reset`))))

(event `self.Box.OnComponentEndOverlap`
  (params (OverlappedComponent :type "PrimitiveComponent Object Reference") (OtherActor :type "Actor Object Reference") (OtherComp :type "PrimitiveComponent Object Reference") (OtherBodyIndex :type Integer))
  (cast `/Game/ThirdPersonBP/Blueprints/ThirdPersonCharacter` OtherActor)
  (`KismetSystemLibrary.Delay` 2.0)
  (`self.Reset`))

(fn `UserConstructionScript`)