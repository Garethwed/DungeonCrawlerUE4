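; Shop NPC actor that opens a shop screen when the third-person character enters its trigger.
; On overlap it blends the player's view to itself, disables the character's movement and switches input to UI only.
; After a short delay it creates the boss token shop widget and shows the mouse cursor.
; It contains no logic for closing the shop or restoring control.
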(event `self.ShopTrigger.OnComponentBeginOverlap`
  (params (OverlappedComponent :type "PrimitiveComponent Object Reference") (OtherActor :type "Actor Object Reference") (OtherComp :type "PrimitiveComponent Object Reference") (OtherBodyIndex :type Integer) (bFromSweep :type Boolean) (SweepResult :type "HitResult Structure (by ref)"))
  (bind _returnvalue (`GameplayStatics.GetPlayerController` 0))
  (bind _asthird_person_character (cast `/Game/ThirdPersonBP/Blueprints/ThirdPersonCharacter` OtherActor))
  (`PlayerController.SetViewTargetWithBlend` (`GameplayStatics.GetPlayerController` 0) self 1.5 "VTBlend_Linear" 0.0 false)
  (`CharacterMovementComponent.DisableMovement` (`Character.CharacterMovement` _asthird_person_character))
  (`WidgetBlueprintLibrary.SetInputMode_UIOnlyEx` _returnvalue null)
  (`KismetSystemLibrary.Delay` 1.0)
  (bind _returnvalue_2 (`|CreateWidget` "/Game/Widgets/UMG_ShopBossToken.UMG_ShopBossToken_C"))
  (`UserWidget.AddToViewport` _returnvalue_2 0)
  (set `PlayerController.bShowMouseCursor` true _returnvalue))

(fn `UserConstructionScript`)