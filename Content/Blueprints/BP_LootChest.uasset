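; BP_LootChest is a loot chest that bursts out physical coins when a ThirdPersonCharacter enters its ChestOpenCollision.
; The overlap spawns a small random number of BP_Coin actors just above the chest, each with a random rotation.
; Each coin gets a random sideways and upward impulse plus an angular impulse for spin.
; Nothing disables the trigger afterward, so every new overlap spawns another batch.
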(event `self.ChestOpenCollision.OnComponentBeginOverlap`
  (params (OverlappedComponent :type "PrimitiveComponent Object Reference") (OtherActor :type "Actor Object Reference") (OtherComp :type "PrimitiveComponent Object Reference") (OtherBodyIndex :type Integer) (bFromSweep :type Boolean) (SweepResult :type "HitResult Structure (by ref)"))
  (bind _returnvalue (`SceneComponent.K2_GetComponentToWorld` (`self.Chest`)))
  (cast `/Game/ThirdPersonBP/Blueprints/ThirdPersonCharacter` OtherActor)
  (for _ (range (+ (`KismetMathLibrary.RandomIntegerInRange` 3 7) 1))
    (bind _returnvalue_2 (`|SpawnActorFromClass` "/Game/Blueprints/BP_Coin.BP_Coin_C" (`KismetMathLibrary.MakeTransform` (`KismetMathLibrary.MakeVector` (.x (.location _returnvalue)) (.y (.location _returnvalue)) (+ (.z (.location _returnvalue)) 100.0)) (`KismetMathLibrary.RandomRotator` false) (.scale _returnvalue)) "Undefined" "OverrideRootScale" null null))
    (`PrimitiveComponent.AddImpulse` (`/Game/Blueprints/BP_Coin.Coin` _returnvalue_2) (`KismetMathLibrary.MakeVector` (`KismetMathLibrary.Conv_IntToDouble` (`KismetMathLibrary.RandomIntegerInRange` -700 700)) (`KismetMathLibrary.Conv_IntToDouble` (`KismetMathLibrary.RandomIntegerInRange` -700 700)) (`KismetMathLibrary.Conv_IntToDouble` (`KismetMathLibrary.RandomIntegerInRange` 500 1200))) "None" false)
    (`PrimitiveComponent.AddAngularImpulseInRadians` (`/Game/Blueprints/BP_Coin.Coin` _returnvalue_2) (0.0 0.0 2000.0) "None" false)))

(fn `UserConstructionScript`)