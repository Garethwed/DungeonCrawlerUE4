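; Weapon chest that sells a random weapon to an overlapping ThirdPersonCharacter through a roulette-style reveal.
; A DoOnce overlap checks Coins, then a delayed loop swaps random weapons above the chest, slowing each step and avoiding most repeats.
; The last pick respawns with an explosion and costs the player one boss token, despite the Coins check.
; Tick advances a yaw that is applied only as each weapon spawns.
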(event `self.ReceiveTick`
  (params (DeltaSeconds :type "Float (single-precision)"))
  (bind (_current_rotation_roll _current_rotation_pitch _current_rotation_yaw) (`KismetMathLibrary.BreakRotator` (`self.Current Rotation`)))
  (bind (_returnvalue_roll _returnvalue_pitch _returnvalue_yaw) (`KismetMathLibrary.BreakRotator` (`KismetMathLibrary.MakeRotator` 0.0 0.0 (* DeltaSeconds (`self.YawPerSecond`)))))
  ;[1 1 1] sets rotation of each weapon
  (set `self.Current Rotation` (`KismetMathLibrary.MakeRotator` 0.0 0.0 (+ _current_rotation_yaw _returnvalue_yaw))))

(event `self.ChestOpenCollision.OnComponentBeginOverlap`
  (params (OverlappedComponent :type "PrimitiveComponent Object Reference") (OtherActor :type "Actor Object Reference") (OtherComp :type "PrimitiveComponent Object Reference") (OtherBodyIndex :type Integer) (bFromSweep :type Boolean) (SweepResult :type "HitResult Structure (by ref)"))
  (bind _indexofrotatingwep (`self.IndexofRotatingWep`))
  (bind _weapons (`self.Weapons`))
  (bind _returnvalue (`SceneComponent.K2_GetComponentToWorld` (`self.Chest`)))
  (bind _output (`|GetArrayItem` _weapons (`self.IndexofRotatingWep`)))
  (bind _returnvalue_2 (* (.scale _returnvalue) (`self.SizeScaleOfWeapon`)))
  (bind _returnvalue_3 (+ (.z (.location _returnvalue)) (`self.DistanceAboveChest`)))
  (`/Engine/EditorBlueprintResources/StandardMacros.DoOnce` false
    (:`Completed`
      (bind _asthird_person_character (cast `/Game/ThirdPersonBP/Blueprints/ThirdPersonCharacter` OtherActor))
      (if (>= (`/Game/ThirdPersonBP/Blueprints/ThirdPersonCharacter.Coins` _asthird_person_character) 1)
        (set `/Game/ThirdPersonBP/Blueprints/ThirdPersonCharacter.OpeningBox` true _asthird_person_character)
        (bind _index (`/Game/Blueprints/CustomLoop.Custom Loop With Delay` 0 (`self.ItemCycleCount`) (`self.DelayBetweenItem`))
          (:`Loop Body`
            (`self.K2_DestroyActor` (`self.RotatingWeapon`))
            (set `self.IndexofRotatingWep` (`KismetMathLibrary.RandomIntegerInRange` 0 (- (`KismetArrayLibrary.Array_Length` _weapons) 1)))
            (if (== (`self.IndexofRotatingWep`) (`self.LastWep`))
              (if (== (`self.IndexofRotatingWep`) 0)
                ;[1 1 1] spawns each weapon to be destroyed for the cycle
                (`/Engine/EditorBlueprintResources/StandardMacros.IncrementInt` _indexofrotatingwep
                  (:`  `
                    _))
                (else
                  (`/Engine/EditorBlueprintResources/StandardMacros.DecrementInt` _indexofrotatingwep
                    (:`  `
                      _)))))
            (bind _returnvalue_4 (`|SpawnActorFromClass` _output (`KismetMathLibrary.MakeTransform` (`KismetMathLibrary.MakeVector` (.x (.location _returnvalue)) (.y (.location _returnvalue)) _returnvalue_3) (`self.Current Rotation`) _returnvalue_2) "Undefined" "OverrideRootScale" null null))
            (set `self.RotatingWeapon` _returnvalue_4)
            (`KismetSystemLibrary.PrintString` (`KismetStringLibrary.Conv_IntToString` _index))
            (set `self.DelayBetweenItem` (* (`self.DelayBetweenItem`) 1.1))
            (set `self.LastWep` (`self.IndexofRotatingWep`)))
          (:`Completed`
            ;[1 1 1] spawns final weapon to be picked up
            (`self.K2_DestroyActor` (`self.RotatingWeapon`))
            (bind _returnvalue_5 (`|SpawnActorFromClass` _output (`KismetMathLibrary.MakeTransform` (`KismetMathLibrary.MakeVector` (.x (.location _returnvalue)) (.y (.location _returnvalue)) _returnvalue_3) (`self.Current Rotation`) _returnvalue_2) "Undefined" "OverrideRootScale" null null))
            (`GameplayStatics.SpawnEmitterAtLocation` "/Game/StarterContent/Particles/P_Explosion.P_Explosion" (`self.K2_GetActorLocation` _returnvalue_5) (`self.K2_GetActorRotation` _returnvalue_5))
            (bind _asthird_person_character_2 (cast `/Game/ThirdPersonBP/Blueprints/ThirdPersonCharacter` (`GameplayStatics.GetPlayerCharacter` 0)))
            (`/Game/ThirdPersonBP/Blueprints/ThirdPersonCharacter.SpendBossTokens` _asthird_person_character_2 1)
            (set `/Game/ThirdPersonBP/Blueprints/ThirdPersonCharacter.OpeningBox` false _asthird_person_character_2)))
        (else
          ;[1 1 1] not enough tokens to buy chest
          (`KismetSystemLibrary.PrintString` "not enough Coins"))))))

(fn `UserConstructionScript`)