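; AI controller for a melee character that wanders the navmesh and chases the player once perceived.
; Wander loops through a random delay and a move to a random nearby navigable point, repeating only on success.
; A successful perception of the ThirdPersonCharacter stores it and starts a fast looping timer that re-issues a move to its location.
; Nothing here sets the SeesPlayer flag that gates wandering or clears the chase timer.
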(event `self.ReceiveBeginPlay`
  (`self.Wander`))

(event `Wander`
  (bind _returnvalue (`self.K2_GetPawn`))
  (`KismetSystemLibrary.Delay` (`KismetMathLibrary.RandomFloatInRange` 1.0 3.0))
  (if (not (`self.SeesPlayer`))
    (`|AIMoveTo` _returnvalue (`NavigationSystemV1.K2_GetRandomLocationInNavigableRadius` (`self.K2_GetActorLocation` _returnvalue) 2000.0 null null) null
      (:`OnSuccess`
        (`self.Wander`)))))

(event `self.AIPerception.OnTargetPerceptionUpdated`
  (params (Actor :type "Actor Object Reference") (Stimulus :type "AIStimulus Structure"))
  (bind _asthird_person_character (cast `/Game/ThirdPersonBP/Blueprints/ThirdPersonCharacter` Actor))
  (set `self.Player` _asthird_person_character)
  (`KismetSystemLibrary.PrintString` "sees player")
  (if (`.bSuccessfullySensed` (break `AIStimulus` Stimulus))
    (`KismetSystemLibrary.K2_SetTimer` null "Chase" 0.05 true)))

(event `Chase`
  (set `self.PlayerLocation` (`self.K2_GetActorLocation` (`self.Player`)))
  (`|AIMoveTo` (`self.K2_GetPawn`) (`self.PlayerLocation`) null))

(fn `UserConstructionScript`
  (`parent.UserConstructionScript`))