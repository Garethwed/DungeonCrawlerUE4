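; Melee enemy AI character that plays a slash montage when a ThirdPersonCharacter enters its Box trigger.
; The overlap stores the player and a DoOnce gates the attack.
; Two seconds after the player exits, Reset reopens the gate, replaying the montage first if the player is back inside.
; DamagePlayer is an empty stub, and debug prints remain in the attack path.
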(event `self.Box.OnComponentBeginOverlap`
  (params (OverlappedComponent :type "PrimitiveComponent Object Reference") (OtherActor :type "Actor Object Reference") (OtherComp :type "PrimitiveComponent Object Reference") (OtherBodyIndex :type Integer) (bFromSweep :type Boolean) (SweepResult :type "HitResult Structure (by ref)"))
  (`KismetSystemLibrary.PrintString` "Hello")
  (bind _asthird_person_character (cast `/Game/ThirdPersonBP/Blueprints/ThirdPersonCharacter` OtherActor))
  (set `self.Player` _asthird_person_character)
  (`/Engine/EditorBlueprintResources/StandardMacros.DoOnce` false :!label _label
    (:`Completed`
      (`AnimInstance.Montage_Play` (`SkeletalMeshComponent.GetAnimInstance` (`self.Mesh`)) "/Game/Blueprints/MeleeAttackAI/Anims/SlashAnimMontage.SlashAnimMontage" 1.0 "MontageLength" 0.0 true)
      (`KismetSystemLibrary.PrintString` "playing montage"))))

(event `DamagePlayer`
  ;[1 1 1] Do damage to player here
)

(event `Reset`
  (if (`PrimitiveComponent.IsOverlappingActor` (`self.Box`) (`self.Player`))
    (`AnimInstance.Montage_Play` (`SkeletalMeshComponent.GetAnimInstance` (`self.Mesh`)) "/Game/Blueprints/MeleeAttackAI/Anims/SlashAnimMontage.SlashAnimMontage" 1.0 "MontageLength" 0.0 true)
    (goto _label :!via `Reset`)
    (else
      (goto _label :!via `Reset`))))

(event `self.Box.OnComponentEndOverlap`
  (params (OverlappedComponent :type "PrimitiveComponent Object Reference") (OtherActor :type "Actor Object Reference") (OtherComp :type "PrimitiveComponent Object Reference") (OtherBodyIndex :type Integer))
  (cast `/Game/ThirdPersonBP/Blueprints/ThirdPersonCharacter` OtherActor)
  (`KismetSystemLibrary.Delay` 2.0)
  (`self.Reset`))

(fn `UserConstructionScript`)